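; BP_Whiteboard is a whiteboard actor that can be drawn on at runtime through a render target.
; On BeginPlay it creates a dynamic instance of M_WhiteboardMarker via the Whiteboard component and clears T_CanvasWhiteboard to black.
; DrawOnWhiteboard passes a 2D location to the marker material and draws it into that render target.
; DrawSize adjusts the brush through the material's Size parameter.
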(event `self.ReceiveBeginPlay`
  (bind _returnvalue (`PrimitiveComponent.CreateDynamicMaterialInstance` (`self.Whiteboard`) 0 "/Game/Whiteboard/M_WhiteboardMarker.M_WhiteboardMarker" "None"))
  (set `self.WhiteBoardMarker` _returnvalue)
  (`KismetRenderingLibrary.ClearRenderTarget2D` "/Game/Whiteboard/T_CanvasWhiteboard.T_CanvasWhiteboard"))

(event `DrawOnWhiteboard`
  (params (LocationToDraw :type "Vector2D Structure"))
  (bind _whiteboardmarker (`self.WhiteBoardMarker`))
  (`MaterialInstanceDynamic.SetVectorParameterValue` _whiteboardmarker "DrawLocation" (`KismetMathLibrary.Conv_VectorToLinearColor` (`KismetMathLibrary.Conv_Vector2DToVector` LocationToDraw 0.1)))
  (`KismetRenderingLibrary.DrawMaterialToRenderTarget` "/Game/Whiteboard/T_CanvasWhiteboard.T_CanvasWhiteboard" _whiteboardmarker))

(event `DrawSize`
  (params (DrawSize :type "Float (double-precision)"))
  (`MaterialInstanceDynamic.SetScalarParameterValue` (`self.WhiteBoardMarker`) "Size" DrawSize))

(fn `UserConstructionScript`)